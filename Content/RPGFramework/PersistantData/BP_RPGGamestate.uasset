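; RPG game state that runs the in-game clock and calendar and looks up saved items.
; Each tick, SetClockwork scales delta time by TimeUnit into a 24-hour ClockWork value, with whole-day overflow stored as DayTick.
; Clock derives seconds, minutes and hours from ClockWork, while Calendar adds DayTick to the date and advances month and year.
; SavedItems searches by object name, returning a found flag and location.
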(event `self.ReceiveBeginPlay`)

(event `self.ReceiveTick`
  (params (DeltaSeconds :type "Float (single-precision)"))
  (`self.SetClockwork` DeltaSeconds)
  (`self.Clock`)
  (`self.Calendar`))

(fn `Calendar`
  (bind (_gametime_timeunit _gametime_clockwork _gametime_seconds _gametime_minutes _gametime_hours _gametime_gametime _gametime_day _gametime_month _gametime_year _gametime_gamedate _gametime_daytick) (break `/Game/RPGFramework/Blueprints/SGameTime` (`self.GameTime`)))
  (bind (_gametime_timeunit_2 _gametime_clockwork_2 _gametime_seconds_2 _gametime_minutes_2 _gametime_hours_2 _gametime_gametime_2 _gametime_day_2 _gametime_month_2 _gametime_year_2 _gametime_gamedate_2 _gametime_daytick_2) (break `/Game/RPGFramework/Blueprints/SGameTime` (`self.GameTime`)))
  (bind (_gametime_timeunit_3 _gametime_clockwork_3 _gametime_seconds_3 _gametime_minutes_3 _gametime_hours_3 _gametime_gametime_3 _gametime_day_3 _gametime_month_3 _gametime_year_3 _gametime_gamedate_3 _gametime_daytick_3) (break `/Game/RPGFramework/Blueprints/SGameTime` (`self.GameTime`)))
  (bind (_gametime_timeunit_4 _gametime_clockwork_4 _gametime_seconds_4 _gametime_minutes_4 _gametime_hours_4 _gametime_gametime_4 _gametime_day_4 _gametime_month_4 _gametime_year_4 _gametime_gamedate_4 _gametime_daytick_4) (break `/Game/RPGFramework/Blueprints/SGameTime` (`self.GameTime`)))
  (bind _returnvalue (+ _gametime_day _gametime_daytick))
  (set `self.GameTime` (make `/Game/RPGFramework/Blueprints/SGameTime` _gametime_timeunit _gametime_clockwork _gametime_seconds _gametime_minutes _gametime_hours _gametime_gametime _returnvalue _gametime_month _gametime_year _gametime_gamedate _gametime_daytick))
  (if (> _returnvalue (`KismetMathLibrary.DaysInMonth` _gametime_year _gametime_month))
    (set `self.GameTime` (make `/Game/RPGFramework/Blueprints/SGameTime` _gametime_timeunit_3 _gametime_clockwork_3 _gametime_seconds_3 _gametime_minutes_3 _gametime_hours_3 _gametime_gametime_3 _gametime_day_3 (+ _gametime_month_3 1) _gametime_year_3 _gametime_gamedate_3 _gametime_daytick_3)))
  (if (> _gametime_month 12)
    (set `self.GameTime` (make `/Game/RPGFramework/Blueprints/SGameTime` _gametime_timeunit_2 _gametime_clockwork_2 _gametime_seconds_2 _gametime_minutes_2 _gametime_hours_2 _gametime_gametime_2 _gametime_day_2 1 (+ _gametime_year_2 1) _gametime_gamedate_2 _gametime_daytick_2))
    (set `self.GameTime` (make `/Game/RPGFramework/Blueprints/SGameTime` 0.0 _gametime_clockwork_4 _gametime_seconds_4 _gametime_minutes_4 _gametime_hours_4 _gametime_gametime_4 _gametime_day_4 _gametime_month_4 _gametime_year_4 (`|MakeArray` _gametime_day_4 _gametime_month_4 _gametime_year_4) _gametime_daytick_4))))

(fn `Clock`
  (bind (_gametime_timeunit _gametime_clockwork) (break `/Game/RPGFramework/Blueprints/SGameTime` (`self.GameTime`)))
  (bind (_gametime_timeunit_2 _gametime_clockwork_2 _gametime_seconds _gametime_minutes _gametime_hours _gametime_gametime _gametime_day _gametime_month _gametime_year _gametime_gamedate _gametime_daytick) (break `/Game/RPGFramework/Blueprints/SGameTime` (`self.GameTime`)))
  (bind (_remainder _returnvalue) (`KismetMathLibrary.FMod` (* _gametime_clockwork 3600.0) 60.0))
  (bind _returnvalue_2 (`KismetMathLibrary.FFloor` _remainder))
  (bind (_remainder_2 _returnvalue_3) (`KismetMathLibrary.FMod` (`KismetMathLibrary.Conv_IntToDouble` _returnvalue) 60.0))
  (bind _returnvalue_4 (`KismetMathLibrary.FFloor` _remainder_2))
  (bind _returnvalue_5 (`KismetMathLibrary.FFloor` (`KismetMathLibrary.FMod` (`KismetMathLibrary.Conv_IntToDouble` _returnvalue_3) 24.0)))
  (set `self.GameTime` (make `/Game/RPGFramework/Blueprints/SGameTime` _gametime_timeunit_2 _gametime_clockwork_2 _returnvalue_2 _returnvalue_4 _returnvalue_5 (`|MakeArray` _returnvalue_2 _returnvalue_4 _returnvalue_5) _gametime_day _gametime_month _gametime_year _gametime_gamedate _gametime_daytick)))

(fn `SavedItems`
  (params (ObjectName :type String))
  (returns (ReturnValue :type Boolean) (Location :type "Transform Structure"))
  (locals (LocalBool :type Boolean))
  (for _array_element _
    (bind (_objectname _location) (break `/Game/RPGFramework/PersistantData/PersistantItemData` _array_element))
    (`KismetSystemLibrary.PrintString` _objectname false false)
    (if (`KismetStringLibrary.EqualEqual_StrStr` ObjectName _objectname)
      (set `local.LocalBool` true)
      (break)))
  (return (`local.LocalBool`) _location))

(fn `SetClockwork`
  (params (`Delta Seconds` :type "Float (double-precision)"))
  (bind (_gametime_timeunit _gametime_clockwork _gametime_seconds _gametime_minutes _gametime_hours _gametime_gametime _gametime_day _gametime_month _gametime_year _gametime_gamedate) (break `/Game/RPGFramework/Blueprints/SGameTime` (`self.GameTime`)))
  (bind (_remainder _returnvalue) (`KismetMathLibrary.FMod` (+ (/ `Delta Seconds` _gametime_timeunit) _gametime_clockwork) 24.0))
  (set `self.GameTime` (make `/Game/RPGFramework/Blueprints/SGameTime` _gametime_timeunit _remainder _gametime_seconds _gametime_minutes _gametime_hours _gametime_gametime _gametime_day _gametime_month _gametime_year _gametime_gamedate _returnvalue)))

(fn `UserConstructionScript`)