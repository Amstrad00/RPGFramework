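; Base NPC character that handles cover, crouching and attacks for AI combat.
; Entering or exiting cover toggles crouch and switches the AI controller between ranged-combat and base behavior trees.
; Melee, ranged and looping timer attacks share one muzzle-to-focus-actor line trace that applies damage, ignoring the stored AttackTarget.
; Tick disables movement-oriented rotation at large control-to-actor yaw differences, and near-miss damage only prints debug text.
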(event `ExitCover`
  (set `self.IsInCover` false)
  (`self.EndCrouch`)
  (bind _asaic_base_npc (cast `/Game/RPGFramework/NPC/AIC_BaseNPC` (`self.GetController`)))
  (`AIController.RunBehaviorTree` _asaic_base_npc "/Game/RPGFramework/NPC/BT_BaseNPC.BT_BaseNPC"))

(event `EnterCover`
  (set `self.IsInCover` true)
  (`self.StartCrouch`)
  (bind _asaic_base_npc (cast `/Game/RPGFramework/NPC/AIC_BaseNPC` (`self.GetController`)))
  (`AIController.RunBehaviorTree` _asaic_base_npc "/Game/RPGFramework/NPC/BT_BaseNPC_RangedCombat.BT_BaseNPC_RangedCombat"))

(event `StartCrouch`
  (`self.Crouch`))

(event `EndCrouch`
  (`self.UnCrouch`)
  (`KismetSystemLibrary.PrintString` "Uncrouched" true true (struct :`R` 1.0 :`G` 0.014998 :`A` 1.0)))

(event `self.ReceiveTick`
  (params (DeltaSeconds :type "Float (single-precision)"))
  (bind _charactermovement (`self.CharacterMovement`))
  (if (>= (`KismetMathLibrary.Abs` (.yaw (`KismetMathLibrary.NormalizedDeltaRotator` (`self.GetControlRotation`) (`self.K2_GetActorRotation`)))) 70.0)
    (set `CharacterMovementComponent.bOrientRotationToMovement` false _charactermovement)
    (else
      (set `CharacterMovementComponent.bOrientRotationToMovement` true _charactermovement))))

(event `self.ReceiveAnyDamage`
  (params (Damage :type "Float (single-precision)") (DamageType :type "DamageType Object Reference") (InstigatedBy :type "Controller Object Reference") (DamageCauser :type "Actor Object Reference"))
  (cast `/Game/RPGFramework/Blueprints/DMG_NearMiss` DamageType)
  (`KismetSystemLibrary.PrintString` "Near Miss" true true (struct :`R` 1.0 :`G` 0.014998 :`A` 1.0)))

(event `Start Attack`
  (`KismetSystemLibrary.K2_SetTimer` null "Attack" 1.0 true))

(event `Attack`
  (bind (_outhit _returnvalue) (`KismetSystemLibrary.LineTraceSingle` :`Start` (`SceneComponent.GetSocketLocation` (`self.Weapon`) "Muzzle") :`End` (`self.K2_GetActorLocation` (`AIController.GetFocusActor` (`AIBlueprintHelperLibrary.GetAIController` (`self.GetController`)))) :`TraceChannel` "TraceTypeQuery1" :`DrawDebugType` "ForDuration"))
  (if _returnvalue
    (`GameplayStatics.ApplyDamage` (`.HitActor` (`GameplayStatics.BreakHitResult` _outhit)) 10.0)))

(event `Stop Attack`
  (`KismetSystemLibrary.K2_ClearTimer` null "Attack"))

(event `/Game/RPGFramework/NPC/Tasks/CombatInterface.MeleeAttack`
  (params (AttackTarget :type "Actor Object Reference"))
  (set `self.AttackTarget` AttackTarget)
  (`|PlayMontage` (`self.Mesh`) "/Game/Mannequin/Animations/ThirdPerson/ThirdPersonAttack_Montage.ThirdPersonAttack_Montage"
    (:`then`
      (`self.Attack`))))

(event `/Game/RPGFramework/NPC/Tasks/CombatInterface.RangedAttack`
  (params (AttackTarget :type "Actor Object Reference"))
  (set `self.AttackTarget` AttackTarget)
  (`|PlayMontage` (`self.Mesh`) "/Game/Mannequin/Animations/AnimStarterPack/Fire_Rifle_Ironsights_Montage.Fire_Rifle_Ironsights_Montage"
    (:`then`
      (`self.Attack`))))

(fn `UserConstructionScript`)