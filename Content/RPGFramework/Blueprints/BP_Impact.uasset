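; BP_Impact is a component that plays an impact sound when its owning actor's static mesh hits something.
; On BeginPlay it binds to the mesh's hit event, then arms the sound after a short delay, apparently to silence hits at spawn.
; Hits above a velocity-difference threshold play the sound at the impact location through a DoOnce gate, which resets after a brief cooldown.
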(event `self.ReceiveBeginPlay`
  (bind _returnvalue (`Actor.GetComponentByClass` (`self.GetOwner`) "/Script/Engine.StaticMeshComponent"))
  (`/Engine/EditorBlueprintResources/StandardMacros.IsValid` _returnvalue
    (:`Is Valid`
      (add `PrimitiveComponent.OnComponentHit` _returnvalue (`|CreateDelegate` :!event `OnComponentHit_Event`))
      (`self.BeginPlayTurnOnsounds`))))

(event `BeginPlayTurnOnsounds`
  (`KismetSystemLibrary.Delay` 1.0)
  (goto _label :!via `Reset`))

(event `OnComponentHit_Event`
  (params (HitComponent :type "PrimitiveComponent Object Reference") (OtherActor :type "Actor Object Reference") (OtherComp :type "PrimitiveComponent Object Reference") (NormalImpulse :type "Vector Structure") (Hit :type "HitResult Structure (by ref)"))
  (bind (_bblockinghit _binitialoverlap _time _location _impactpoint _normal _impactnormal _physmat _hitactor _hitcomponent) (`GameplayStatics.BreakHitResult` Hit))
  (if (> (`KismetMathLibrary.VSize` (- (`SceneComponent.GetComponentVelocity` HitComponent) (`SceneComponent.GetComponentVelocity` _hitcomponent))) 20.0)
    (`|ExecutionSequence`
      (:`then_1`
        (`/Engine/EditorBlueprintResources/StandardMacros.DoOnce` true :!label _label
          (:`Completed`
            (`GameplayStatics.PlaySoundAtLocation` (`self.ImpactSound`) _location (struct) (`self.Volume`))
            (`KismetSystemLibrary.Delay` 0.5)
            (goto _label :!via `Reset`)))))))