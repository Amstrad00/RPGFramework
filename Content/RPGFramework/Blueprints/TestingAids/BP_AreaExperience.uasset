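; BP_AreaExperience is a testing-aid actor that grants experience repeatedly while something overlaps its sphere.
; Overlap begin starts a looping three-second timer on the Experience function, and overlap end clears it.
; Experience calls HandleXP on player character 0 with ExperienceAmount, ignoring the stored ExperienceTarget, so any overlapping actor triggers XP for that player.
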(event `self.Sphere.OnComponentBeginOverlap`
  (params (OverlappedComponent :type "PrimitiveComponent Object Reference") (OtherActor :type "Actor Object Reference") (OtherComp :type "PrimitiveComponent Object Reference") (OtherBodyIndex :type Integer) (bFromSweep :type Boolean) (SweepResult :type "HitResult Structure (by ref)"))
  (set `self.ExperienceTarget` OtherActor)
  (bind _returnvalue (`KismetSystemLibrary.K2_SetTimer` self "Experience" 3.0 true))
  (`KismetSystemLibrary.PrintString` "Giving Experience"))

(event `self.Sphere.OnComponentEndOverlap`
  (params (OverlappedComponent :type "PrimitiveComponent Object Reference") (OtherActor :type "Actor Object Reference") (OtherComp :type "PrimitiveComponent Object Reference") (OtherBodyIndex :type Integer))
  (`KismetSystemLibrary.K2_ClearAndInvalidateTimerHandle` (stale `self.Sphere.OnComponentBeginOverlap` _returnvalue)))

(fn `Experience`
  (bind _asbp_playercharacter (cast `/Game/RPGFramework/Blueprints/BP_Playercharacter` (`GameplayStatics.GetPlayerCharacter` 0)))
  (`/Game/RPGFramework/Blueprints/BP_Playercharacter.HandleXP` _asbp_playercharacter (`self.ExperienceAmount`)))

(fn `UserConstructionScript`)