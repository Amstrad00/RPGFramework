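; BP_BasicProjectile is a projectile actor that plays surface-specific impact effects when it hits something, then destroys itself.
; Its Sphere hit event reads the physical surface type from the first material on the struck component.
; That type selects the sound, decal and particle emitter spawned at the impact point, with metal as the default and a separate flesh set.
; The decal is oriented from the hit normal, with pitch flipped 180 degrees.
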(event `self.Sphere.OnComponentHit`
  (params (HitComponent :type "PrimitiveComponent Object Reference") (OtherActor :type "Actor Object Reference") (OtherComp :type "PrimitiveComponent Object Reference") (NormalImpulse :type "Vector Structure") (Hit :type "HitResult Structure (by ref)"))
  (bind (_bblockinghit _binitialoverlap _time _distance _location _impactpoint _normal _impactnormal _physmat _hitactor _hitcomponent) (`GameplayStatics.BreakHitResult` Hit))
  (bind (_returnvalue_roll _returnvalue_pitch _returnvalue_yaw) (`KismetMathLibrary.BreakRotator` (`KismetMathLibrary.MakeRotFromX` _normal)))
  (bind _surfacetype (`PhysicalMaterial.SurfaceType` (`MaterialInterface.GetPhysicalMaterial` (`PrimitiveComponent.GetMaterial` _hitcomponent 0))))
  (`GameplayStatics.PlaySoundAtLocation` (select `EPhysicalSurface` _surfacetype :`SurfaceType_Default` "/Game/RPGFramework/Sounds/impact_metal_cue.impact_metal_Cue" :`SurfaceType1` "/Game/RPGFramework/Sounds/impact_metal_cue.impact_metal_Cue" :`SurfaceType2` "/Game/RPGFramework/Sounds/impact_flesh_Cue.impact_flesh_Cue" :!type "SoundBase Object Reference") _location)
  (`GameplayStatics.SpawnDecalAtLocation` (select `EPhysicalSurface` _surfacetype :`SurfaceType_Default` "/Game/RPGFramework/Materials/Impact_Metal_Mat.Impact_Metal_Mat" :`SurfaceType1` "/Game/RPGFramework/Materials/Impact_Metal_Mat.Impact_Metal_Mat" :`SurfaceType2` "/Game/RPGFramework/Materials/Impact_Flesh_Mat.Impact_Flesh_Mat" :!type "MaterialInterface Object Reference") (5.0 5.0 5.0) _location (`KismetMathLibrary.MakeRotator` _returnvalue_roll (+ _returnvalue_pitch 180.0) _returnvalue_yaw))
  (`GameplayStatics.SpawnEmitterAtLocation` (select `EPhysicalSurface` _surfacetype :`SurfaceType_Default` "/Game/RPGFramework/Particles/P_Impact_Sparks.P_Impact_Sparks" :`SurfaceType1` "/Game/RPGFramework/Particles/P_Impact_Sparks.P_Impact_Sparks" :`SurfaceType2` "/Game/RPGFramework/Particles/P_body_bullet_impact.P_body_bullet_impact" :!type "ParticleSystem Object Reference") _location)
  (`self.K2_DestroyActor`))

(fn `UserConstructionScript`)